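; BP_SplineForward is a track segment for game mode 2 that moves the Fox along its spline at a speed driven by typing WPM, destroying itself in other modes.
; BeginPlay scatters random fruit along the spline and starts movement on segment 1.
; A Timeline drives position, reversal and idle/gallop animation.
; Near the end it flags direction waiting, then hands off to a BP_SplineTurn, or halts and resets typing at dead ends.
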(event Custom|FReverse
  (bind _fox (Variables|Default|Getfox))
  (Variables|/Script/UMG.EditableText|SetIsReadOnly (Variables|/Game/HUD/TouchTypingTextInput/WBP_TouchTypingTextInput.WBP_TouchTypingTextInput_C|GetRawInput (Variables|Default|GetWBPTouchTyping)) false)
  (Variables|/Script/FoxRacing.TextBox|Setstop (Utilities|ResolveSoftReference (Variables|Default|Gettextbox)) false)
  (bind _output_get (Variables|Default|Setreverse (not (Variables|Default|Getreverse))))
  (if _output_get
    (bind _track (Timeline|Timeline Reverse)
      (:Update
        (CallFunction|FReset)
        (CallFunction|UpdateNavSys)
        (Transformation|SetActorTransform (Utilities|ResolveSoftReference _fox) (Math|Transform|MakeTransform (Spline|GetLocationatDistanceAlongSpline (Variables|Default|GetSpline) (Math|Float|Lerp 0.0 (Spline|GetSplineLength (Variables|Default|GetSpline)) _track) "World") (Spline|GetRotationatDistanceAlongSpline (Variables|Default|GetSpline) (Math|Float|Lerp 0.0 (Spline|GetSplineLength (Variables|Default|GetSpline)) _track) "World") "1.000000,1.000000,1.000000"))
        (if (Variables|Default|Getreverse)
          (Class|Actor|AddActorWorldRotation (Utilities|ResolveSoftReference _fox) "0.000000,180.000000,0.000000"))
        (CallFunction|Update))
      (:Finished
        (Variables|/Script/FoxRacing.Fox|SetdirSelected (Utilities|ResolveSoftReference _fox) false)
        (Variables|/Script/FoxRacing.Fox|SetdirWaiting (Utilities|ResolveSoftReference _fox) false)
        (bind _returnvalue (Class|SplineForward|GetIDatDir (Variables|/Script/FoxRacing.Fox|GetDir (Utilities|ResolveSoftReference _fox))))
        (if (Math|Conversions|ToBoolean(Integer) _returnvalue)
          (bind _returnvalue_2 (Class|SplineForward|CreateSplineTurn (Variables|Default|GetID) _returnvalue))
          (bind _asbp_spline_turn (Utilities|Casting|CastToBP_SplineTurn _returnvalue_2))
          (Variables|/Script/FoxRacing.Fox|Setforward (Utilities|ResolveSoftReference _fox) false)
          (Variables|/Game/Blueprints/BP_Fox.BP_Fox_C|SetCrtTurn (Utilities|ResolveSoftReference _fox) _asbp_spline_turn)
          (Default|Move _asbp_spline_turn))))
    (else
      (Timeline|Timeline Play))))

(event Custom|Move
  (bind _fox (Variables|Default|Getfox))
  (bind _fox_2 (Variables|Default|Getfox))
  (Development|PrintText (Utilities|Text|ToText(Boolean) (Variables|Default|Getreverse)))
  (Variables|/Game/Blueprints/BP_Fox.BP_Fox_C|SetCrtForward (Utilities|ResolveSoftReference _fox) self)
  (Variables|/Script/FoxRacing.Fox|Setforward (Utilities|ResolveSoftReference _fox) true)
  (if (Variables|Default|Getreverse)
    (bind _track (Timeline|Timeline ReverseFromEnd)
      (:Update
        (CallFunction|FReset)
        (CallFunction|UpdateNavSys)
        (Transformation|SetActorTransform (Utilities|ResolveSoftReference _fox_2) (Math|Transform|MakeTransform (Spline|GetLocationatDistanceAlongSpline (Variables|Default|GetSpline) (Math|Float|Lerp 0.0 (Spline|GetSplineLength (Variables|Default|GetSpline)) _track) "World") (Spline|GetRotationatDistanceAlongSpline (Variables|Default|GetSpline) (Math|Float|Lerp 0.0 (Spline|GetSplineLength (Variables|Default|GetSpline)) _track) "World") "1.000000,1.000000,1.000000"))
        (if (Variables|Default|Getreverse)
          (Class|Actor|AddActorWorldRotation (Utilities|ResolveSoftReference _fox_2) "0.000000,180.000000,0.000000"))
        (CallFunction|Update))
      (:Finished
        (Variables|/Script/FoxRacing.Fox|SetdirSelected (Utilities|ResolveSoftReference _fox_2) false)
        (Variables|/Script/FoxRacing.Fox|SetdirWaiting (Utilities|ResolveSoftReference _fox_2) false)
        (bind _returnvalue (Class|SplineForward|GetIDatDir (Variables|/Script/FoxRacing.Fox|GetDir (Utilities|ResolveSoftReference _fox_2))))
        (if (Math|Conversions|ToBoolean(Integer) _returnvalue)
          (bind _returnvalue_2 (Class|SplineForward|CreateSplineTurn (Variables|Default|GetID) _returnvalue))
          (bind _asbp_spline_turn (Utilities|Casting|CastToBP_SplineTurn _returnvalue_2))
          (Variables|/Script/FoxRacing.Fox|Setforward (Utilities|ResolveSoftReference _fox_2) false)
          (Variables|/Game/Blueprints/BP_Fox.BP_Fox_C|SetCrtTurn (Utilities|ResolveSoftReference _fox_2) _asbp_spline_turn)
          (Default|Move _asbp_spline_turn))))
    (else
      (Timeline|Timeline PlayFromStart))))

(event Custom|Update%20NavSys
  (bind _reverse (Variables|Default|Getreverse))
  (bind _fox (Variables|Default|Getfox))
  (bind _returnvalue (Math|Conversions|ToFloat(Boolean) _reverse))
  (bind _returnvalue_2 (- _returnvalue 0.7))
  (bind _returnvalue_3 (Math|Float|Absolute(Float) _returnvalue_2))
  (bind _returnvalue_4 (Class|SplineForward|GetIDatDir (Variables|/Script/FoxRacing.Fox|GetDir (Utilities|ResolveSoftReference _fox))))
  (if (Math|Conversions|ToBoolean(Integer) _returnvalue_4)
    (if (Variables|Default|Getreverse)
      (if (>= _returnvalue_3 (stale Custom|FReverse _track))
        (Variables|/Script/FoxRacing.Fox|SetdirWaiting (Utilities|ResolveSoftReference _fox) true :!label _label)
        (else
          (Variables|/Script/FoxRacing.Fox|SetdirWaiting (Utilities|ResolveSoftReference _fox) false :!label _label_2)
          (Variables|/Script/FoxRacing.Fox|SetdirSelected (Utilities|ResolveSoftReference _fox) false)))
      (elif (>= (stale Custom|FReverse _track) _returnvalue_3)
        (goto _label)
        (else
          (goto _label_2))))
    (else
      (goto _label_2))))

(event Custom|FReset
  (bind _timeline (Variables|Default|GetTimeline))
  (bind _returnvalue (Components|Animation|GetPlayRate _timeline))
  (bind _returnvalue_2 (/ 1.0 _returnvalue))
  (bind _returnvalue_3 (* 15.0 _returnvalue_2))
  (bind _returnvalue_4 (/ 1.0 _returnvalue_3))
  (if (Variables|Default|Getreverse)
    (if (and (not (Math|Conversions|ToBoolean(Integer) (stale Custom|Update%20NavSys _returnvalue_4))) (>= _returnvalue_4 (stale Custom|FReverse _track)))
      (Components|Timeline|SetPlayRate (Variables|Default|GetTimeline) 0.0 :!label _label)
      (Class|TextBox|Reset (Utilities|ResolveSoftReference (Variables|Default|Gettextbox)))
      (Variables|/Script/UMG.EditableText|SetIsReadOnly (Variables|/Game/HUD/TouchTypingTextInput/WBP_TouchTypingTextInput.WBP_TouchTypingTextInput_C|GetRawInput (Variables|Default|GetWBPTouchTyping)) true)
      (Components|Animation|PlayAnimation (Variables|/Game/Blueprints/BP_Fox.BP_Fox_C|GetSkeletalMesh (Utilities|ResolveSoftReference (Variables|Default|Getfox))) "/Game/Meshes/Fox/Fox_Anim_AnimalArmature_Idle_AnimalArmature.Fox_Anim_AnimalArmature_Idle_AnimalArmature" true)
      (Variables|Default|Setanim1 false)
      (Variables|Default|Setanim2 true))
    (elif (and (not (Math|Conversions|ToBoolean(Integer) (stale Custom|Update%20NavSys _returnvalue_4))) (>= (stale Custom|FReverse _track) (- 1.0 _returnvalue_4)))
      (goto _label))))

(event Custom|FruitSpawn
  (for _index (range 1 (Math|Random|RandomIntegerinRange 1 (Math|Float|Truncate (/ (Spline|GetSplineLength (Variables|Default|GetSpline)) 2e+03))))
    (CallFunction|MakeFruit))
  (Development|PrintString (Utilities|String|ToString(Integer) _index) true true "(R=0.000000,G=0.660000,B=1.000000,A=1.000000)" 2e+01))

(event Custom|Make%20Fruit
  (Game|SpawnActorfromClass "/Game/Blueprints/BP_Fruit.BP_Fruit_C" (Math|Conversions|ToTransform(Vector) (Spline|GetLocationatDistanceAlongSpline (Variables|Default|GetSpline) (Math|Float|Lerp 0.0 (Spline|GetSplineLength (Variables|Default|GetSpline)) (Math|Random|RandomFloatinRange 0.0 1.0)) "World")) "Undefined" "MultiplyWithRoot" 0 (Math|Random|RandomIntegerinRange 1 6) 0))

(event Custom|Update
  (bind _textbox (Variables|Default|Gettextbox))
  (bind _fox (Variables|Default|Getfox))
  (bind _output (Utilities|ResolveSoftReference _textbox))
  (bind _output_2 (Utilities|ResolveSoftReference _fox))
  (bind _wpm (Variables|/Script/FoxRacing.TextBox|GetWPM _output))
  (if (Variables|/Script/FoxRacing.TextBox|Getstop (Utilities|ResolveSoftReference _textbox))
    _
    (else
      (bind _returnvalue (Class|Spline|GetSpeed _wpm))
      (Components|Timeline|SetPlayRate (Variables|Default|GetTimeline) (/ (* _wpm _returnvalue) (Spline|GetSplineLength (Variables|Default|GetSpline))))))
  (if (< _wpm 1e+01)
    (if (Variables|Default|Getanim1)
      (Components|Animation|PlayAnimation (Variables|/Game/Blueprints/BP_Fox.BP_Fox_C|GetSkeletalMesh _output_2) "/Game/Meshes/Fox/Fox_Anim_AnimalArmature_Idle_AnimalArmature.Fox_Anim_AnimalArmature_Idle_AnimalArmature" true)
      (Variables|Default|Setanim1 false)
      (Variables|Default|Setanim2 true))
    (elif (Variables|Default|Getanim2)
      (Components|Animation|PlayAnimation (Variables|/Game/Blueprints/BP_Fox.BP_Fox_C|GetSkeletalMesh _output_2) "/Game/Meshes/Fox/Fox_Anim_AnimalArmature_Gallop_AnimalArmature.Fox_Anim_AnimalArmature_Gallop_AnimalArmature" true)
      (Variables|Default|Setanim1 true)
      (Variables|Default|Setanim2 false))))

(event EventBeginPlay
  (bind _asbp_game_progress (Utilities|Casting|CastToBP_GameProgress (Game|GetGameInstance)))
  (if (== (Variables|/Game/Blueprints/BP_GameProgress.BP_GameProgress_C|Getmode _asbp_game_progress) 2)
    (Variables|Default|Setspl (Variables|Default|GetSpline))
    (CallFunction|FruitSpawn)
    (if (== 1 (Variables|Default|GetID))
      (Variables|Default|Setreverse false)
      (Variables|Default|Setanim1 true)
      (Variables|Default|Setanim2 true)
      (bind _foundwidgets (Widget|GetAllWidgetsOfClass "/Game/HUD/TouchTypingTextInput/WBP_TouchTypingTextInput.WBP_TouchTypingTextInput_C" true))
      (Variables|Default|SetWBPTouchTyping (Utilities|Array|Get(acopy) _foundwidgets))
      (CallFunction|Move))
    (else
      (Actor|DestroyActor))))

(fn ConstructionScript)

(fn NewFunction)