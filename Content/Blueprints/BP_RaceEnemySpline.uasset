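; Drives the animal opponent in a typing race along a spline, active only when level and race mode match, otherwise destroyed.
; A looping timeline moves Enemy, with play rate and idle or gallop animation following its WPM.
; ChangeToWpm rubber-bands that WPM against the fox's lap and distance, using a per-level baseline plus random jitter.
; Completing all laps shows the race widget's lose state and stops the fox.
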(event Custom|Move
  (bind _newtrack_0 (Timeline|Timeline PlayFromStart)
    (:Update
      (Variables|Default|SetTrack _newtrack_0)
      (Transformation|SetActorTransform (Utilities|ResolveSoftReference (Variables|Default|GetEnemy)) (Math|Transform|MakeTransform (Spline|GetLocationatDistanceAlongSpline (Variables|Default|GetSpline) (Math|Float|Lerp 0.0 (Spline|GetSplineLength (Variables|Default|GetSpline)) _newtrack_0) "World") (Spline|GetRotationatDistanceAlongSpline (Variables|Default|GetSpline) (Math|Float|Lerp 0.0 (Spline|GetSplineLength (Variables|Default|GetSpline)) _newtrack_0) "World") "1.000000,1.000000,1.000000")))
    (:Finished
      (bind _result (Math|Integer|IncrementInt (Variables|Components|GetloopCounter))
        (:%20%20
          (if (and (< _result (Variables|Components|Getlaps)) (not (Variables|Default|Getstop)))
            (CallFunction|Move)
            (else
              (bind _foundwidgets (Widget|GetAllWidgetsOfClass "/Game/HUD/TouchTypingTextInput/WBP_TouchTypingTextInput.WBP_TouchTypingTextInput_C" true))
              (Variables|/Script/UMG.Widget|SetVisibility (Utilities|Array|Get(acopy) _foundwidgets) "Collapsed")
              (Class|TextBox|Reset (Utilities|ResolveSoftReference (Variables|Default|Gettext%20box)))
              (bind _foundwidgets_2 (Widget|GetAllWidgetsOfClass "/Game/HUD/Race/WBP_Race.WBP_Race_C" true))
              (Default|Lose (Utilities|Array|Get(acopy) _foundwidgets_2))
              (Variables|/Script/UMG.Widget|SetVisibility (Utilities|Array|Get(acopy) _foundwidgets_2) "Visible")
              (Default|Lose (Variables|Default|Getfoxspline))
              (Variables|Default|Setwpm 0.0))))))))

(event Custom|BeginEnemy
  (switch int (Variables|/Game/Blueprints/BP_GameProgress.BP_GameProgress_C|Getlevel (stale EventBeginPlay _asbp_game_progress))
    (:1
      (bind _output_get (Variables|Default|Setminwpm 45.0))
      (Variables|Default|Setwpm _output_get))
    (:2
      (bind _output_get_2 (Variables|Default|Setminwpm 55.0))
      (Variables|Default|Setwpm _output_get_2))
    (:3
      (bind _output_get_3 (Variables|Default|Setminwpm 6e+01))
      (Variables|Default|Setwpm _output_get_3))
    (:4
      (bind _output_get_4 (Variables|Default|Setminwpm 65.0))
      (Variables|Default|Setwpm _output_get_4))
    (:5
      (bind _output_get_5 (Variables|Default|Setminwpm 75.0))
      (Variables|Default|Setwpm _output_get_5))
    (:6
      (bind _output_get_6 (Variables|Default|Setminwpm 85.0))
      (Variables|Default|Setwpm _output_get_6)))
  (Variables|Default|Setwpm 0.0)
  (bind _returnvalue (UserInterface|CreateWidget "/Game/HUD/Race/WBP_Race.WBP_Race_C"))
  (UserInterface|Viewport|AddtoViewport _returnvalue 0)
  (Components|Timeline|SetPlayRate (Variables|Default|GetTimeline) 0.0)
  (CallFunction|Move))

(event Custom|ChangeToWpm
  (bind _foxspline (Variables|Default|Getfoxspline))
  (bind _track (Variables|Default|GetTrack))
  (bind _minwpm (Variables|Default|Getminwpm))
  (bind _loopcounter (Variables|Components|GetloopCounter))
  (bind _spline (Variables|Default|GetSpline))
  (bind _returnvalue (Spline|GetSplineLength _spline))
  (bind _returnvalue_2 (/ _minwpm 5.0))
  (bind _foxtrack (Variables|/Game/Blueprints/BP_RaceFoxSpline.BP_RaceFoxSpline_C|Getfoxtrack _foxspline))
  (bind _loopcounter_2 (Variables|/Game/Blueprints/BP_RaceFoxSpline.BP_RaceFoxSpline_C|GetloopCounter _foxspline))
  (bind _spline_2 (Variables|/Game/Blueprints/BP_RaceFoxSpline.BP_RaceFoxSpline_C|GetSpline _foxspline))
  (bind _returnvalue_3 (Math|Float|Lerp 0.0 _returnvalue _track))
  (bind _returnvalue_4 (Spline|GetSplineLength _spline_2))
  (bind _returnvalue_5 (Math|Float|Lerp 0.0 _returnvalue_4 _foxtrack))
  (bind _returnvalue_6 (- _returnvalue_3 _returnvalue_5))
  (if (not (Variables|Default|Getstop))
    (Development|PrintString (Utilities|String|ToString(Float) (Variables|Default|Getwpm)))
    (if (== _loopcounter_2 _loopcounter)
      (if (> (Math|Float|Absolute(Float) _returnvalue_6) 7e+02)
        (Variables|Default|Setwpm (Math|Float|Max(Float) (Variables|/Script/FoxRacing.TextBox|GetWPM (Utilities|ResolveSoftReference (Variables|Default|Gettext%20box))) _minwpm))
        (if (> _returnvalue_6 0.0)
          (Variables|Default|Setwpm (+ (Variables|Default|Getwpm) (* _returnvalue_2 -1.0)) :!label _label)
          (else
            (Variables|Default|Setwpm (+ (Variables|Default|Getwpm) _returnvalue_2) :!label _label_2))))
      (elif (> _loopcounter_2 _loopcounter)
        (goto _label_2)
        (else
          (goto _label))))
    (Variables|Default|Setwpm (Math|Float|Min(Float) (Math|Float|Max(Float) (+ (Variables|Default|Getwpm) (Math|Random|RandomFloatinRange -4.0 7.0)) 0.0) (+ (Variables|Default|Getminwpm) 5.0)))
    (Development|PrintString "ENEMY SPEED UPDATED")
    (Utilities|Time|SetTimerbyFunctionName 0 "ChangeToWpm" 2.0)))

(event Custom|Update
  (bind _wpm (Variables|Default|Getwpm))
  (if (Variables|Default|Getstop)
    _
    (else
      (bind _returnvalue (Class|RaceEnemySpline|GetSpeed _wpm))
      (Components|Timeline|SetPlayRate (Variables|Default|GetTimeline) (/ (* _wpm _returnvalue) (Spline|GetSplineLength (Variables|Default|GetSpline))))))
  (if (< _wpm 1e+01)
    (if (Variables|Default|Getanim1)
      (CallFunction|AddIdleAnim)
      (Variables|Default|Setanim1 false)
      (Variables|Default|Setanim2 true))
    (elif (Variables|Default|Getanim2)
      (CallFunction|AddGallopAnim)
      (Variables|Default|Setanim1 true)
      (Variables|Default|Setanim2 false)))
  (Utilities|Time|SetTimerbyFunctionName 0 "Update" 0.5))

(event Custom|AddIdleAnim
  (bind _enemy (Variables|Default|GetEnemy))
  (bind _output (Utilities|ResolveSoftReference _enemy))
  (switch int (Variables|/Game/Blueprints/BP_GameProgress.BP_GameProgress_C|Getlevel (stale EventBeginPlay _asbp_game_progress))
    (:1
      (Components|Animation|PlayAnimation (Variables|/Game/Blueprints/BP_Enemy.BP_Enemy_C|GetDonkey _output) "/Game/Meshes/Donkey/Donkey_Anim_Idle.Donkey_Anim_Idle" true))
    (:2
      (Components|Animation|PlayAnimation (Variables|/Game/Blueprints/BP_Enemy.BP_Enemy_C|GetHorse _output) "/Game/Meshes/Horse/Horse_Anim_AnimalArmature_Idle.Horse_Anim_AnimalArmature_Idle" true))
    (:3
      (Components|Animation|PlayAnimation (Variables|/Game/Blueprints/BP_Enemy.BP_Enemy_C|GetHusky _output) "/Game/Meshes/Husky/Husky_Anim_AnimalArmature_Idle.Husky_Anim_AnimalArmature_Idle" true))
    (:4
      (Components|Animation|PlayAnimation (Variables|/Game/Blueprints/BP_Enemy.BP_Enemy_C|GetDeer _output) "/Game/Meshes/Deer/Deer_Anim_AnimalArmature_Idle.Deer_Anim_AnimalArmature_Idle" true))
    (:5
      (Components|Animation|PlayAnimation (Variables|/Game/Blueprints/BP_Enemy.BP_Enemy_C|GetStag _output) "/Game/Meshes/Stag/tests_Anim_AnimalArmature_AnimalArmature_Idle_Headlow.tests_Anim_AnimalArmature_AnimalArmature_Idle_Headlow" true))
    (:6
      (Components|Animation|PlayAnimation (Variables|/Game/Blueprints/BP_Enemy.BP_Enemy_C|GetWolf _output) "/Game/Meshes/Wolf/Wolf_Anim_AnimalArmature_Idle.Wolf_Anim_AnimalArmature_Idle" true))))

(event Custom|AddGallopAnim
  (bind _enemy (Variables|Default|GetEnemy))
  (bind _output (Utilities|ResolveSoftReference _enemy))
  (switch int (Variables|/Game/Blueprints/BP_GameProgress.BP_GameProgress_C|Getlevel (stale EventBeginPlay _asbp_game_progress))
    (:1
      (Components|Animation|PlayAnimation (Variables|/Game/Blueprints/BP_Enemy.BP_Enemy_C|GetDonkey _output) "/Game/Meshes/Donkey/Donkey_Anim_Gallop.Donkey_Anim_Gallop" true))
    (:2
      (Components|Animation|PlayAnimation (Variables|/Game/Blueprints/BP_Enemy.BP_Enemy_C|GetHorse _output) "/Game/Meshes/Horse/Horse_Anim_Gallop.Horse_Anim_Gallop" true))
    (:3
      (Components|Animation|PlayAnimation (Variables|/Game/Blueprints/BP_Enemy.BP_Enemy_C|GetHusky _output) "/Game/Meshes/Husky/Husky_Anim_Gallop.Husky_Anim_Gallop" true))
    (:4
      (Components|Animation|PlayAnimation (Variables|/Game/Blueprints/BP_Enemy.BP_Enemy_C|GetDeer _output) "/Game/Meshes/Deer/Deer_Anim_Gallop.Deer_Anim_Gallop" true))
    (:5
      (Components|Animation|PlayAnimation (Variables|/Game/Blueprints/BP_Enemy.BP_Enemy_C|GetStag _output) "/Game/Meshes/Stag/tests_Anim_AnimalArmature_AnimalArmature_Gallop.tests_Anim_AnimalArmature_AnimalArmature_Gallop" true))
    (:6
      (Components|Animation|PlayAnimation (Variables|/Game/Blueprints/BP_Enemy.BP_Enemy_C|GetWolf _output) "/Game/Meshes/Wolf/Wolf_Anim_Gallop.Wolf_Anim_Gallop" true))))

(event Custom|Lose
  (Variables|Default|Setstop true)
  (CallFunction|AddIdleAnim)
  (Components|Timeline|SetPlayRate (Variables|Default|GetTimeline) 0.0)
  (Variables|Default|Setwpm 0.0))

(event Collision|EventActorBeginOverlap
  (params (OtherActor :type Actor%20Object%20Reference)))

(event EventBeginPlay
  (Utilities|Time|SetTimerbyFunctionName 0 "Update" 0.5 true)
  (bind _asbp_game_progress (Utilities|Casting|CastToBP_GameProgress (Game|GetGameInstance)))
  (if (and (== (Variables|/Game/Blueprints/BP_GameProgress.BP_GameProgress_C|Getlevel _asbp_game_progress) (Variables|Default|GetID)) (== (Variables|/Game/Blueprints/BP_GameProgress.BP_GameProgress_C|Getmode _asbp_game_progress) 1))
    (CallFunction|BeginEnemy)
    (else
      (Actor|DestroyActor))))

(fn ConstructionScript)