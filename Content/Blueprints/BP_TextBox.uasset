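; BP_TextBox runs the touch-typing input and lesson flow, reading mode and lesson from BP_GameProgress.
; It creates the typing input widget and, outside mode 3, records peak WPM there on a looping timer.
; It drives key highlights and per-hand finger markers on the existing WBP_RobotTextBox.
; Finishing a lesson prints robot text, hides input and clears highlights, advancing progress only if mistakes stay under the limit.
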(event Custom|LessonBeginPlay
  (Variables|Default|Setstop true)
  (Variables|/Script/UMG.Widget|SetVisibility (stale EventBeginPlay _returnvalue) "Collapsed")
  (Class|TextBox|LessonExercises (Variables|Default|GetCrtLesson)))

(event Custom|WorldBeginPlay
  (Default|BeginPlay (stale EventBeginPlay _returnvalue)))

(event Custom|Update
  (Variables|/Game/Blueprints/BP_GameProgress.BP_GameProgress_C|Setmaxwpm (stale EventBeginPlay _asbp_game_progress) (Math|Integer|Max(Integer) (Variables|/Game/Blueprints/BP_GameProgress.BP_GameProgress_C|Getmaxwpm (stale EventBeginPlay _asbp_game_progress)) (Math|Float|Truncate (Variables|Default|GetWPM)))))

(event EventBeginPlay
  (bind _asbp_game_progress (Utilities|Casting|CastToBP_GameProgress (Game|GetGameInstance)))
  (if (!= (Variables|/Game/Blueprints/BP_GameProgress.BP_GameProgress_C|Getmode _asbp_game_progress) 3)
    (Utilities|Time|SetTimerbyFunctionName 0 "Update" 2.0 true))
  (bind _output_get (Variables|Default|SetCrtLesson (- (Variables|/Game/Blueprints/BP_GameProgress.BP_GameProgress_C|Getlesson _asbp_game_progress) 1)))
  (Variables|Default|Setknowledge (- _output_get 1))
  (Variables|Default|SetMode (Variables|/Game/Blueprints/BP_GameProgress.BP_GameProgress_C|Getmode _asbp_game_progress))
  (bind _returnvalue (UserInterface|CreateWidget "/Game/HUD/TouchTypingTextInput/WBP_TouchTypingTextInput.WBP_TouchTypingTextInput_C"))
  (UserInterface|Viewport|AddtoViewport _returnvalue 0)
  (if (== (Variables|/Game/Blueprints/BP_GameProgress.BP_GameProgress_C|Getmode _asbp_game_progress) 1)
    (Variables|/Script/UMG.Widget|SetVisibility _returnvalue "Collapsed"))
  (bind _foundwidgets (Widget|GetAllWidgetsOfClass "/Game/HUD/RobotTextBox/WBP_RobotTextBox.WBP_RobotTextBox_C" true))
  (Variables|Default|SetWBPRobotText (Utilities|Array|Get(acopy) _foundwidgets)))

(event EventColorKey
  (params (Key :type String))
  (bind _wbprobottext (Variables|Default|GetWBPRobotText))
  (bind _lfinger (Variables|Default|Getlfinger))
  (bind _rfinger (Variables|Default|Getrfinger))
  (bind _lfingerselect (Variables|/Game/HUD/RobotTextBox/WBP_RobotTextBox.WBP_RobotTextBox_C|GetLFingerSelect _wbprobottext))
  (bind _rfingerselect (Variables|/Game/HUD/RobotTextBox/WBP_RobotTextBox.WBP_RobotTextBox_C|GetRFingerSelect _wbprobottext))
  (Default|ColorKey _wbprobottext Key)
  (if (Math|Conversions|ToBoolean(Integer) _lfinger)
    (Variables|/Script/UMG.Widget|SetVisibility _lfingerselect "Visible")
    (bind _returnvalue (Class|TextBox|GetFingerPosX false _lfinger))
    (bind _returnvalue_2 (Class|TextBox|GetFingerPosY false _lfinger))
    (Class|CanvasPanelSlot|SetPosition (Class|WidgetLayoutLibrary|SlotasCanvasSlot _lfingerselect) (Math|Vector2D|MakeVector2D (Math|Conversions|ToFloat(Integer) _returnvalue) (Math|Conversions|ToFloat(Integer) _returnvalue_2)))
    (else
      (Variables|/Script/UMG.Widget|SetVisibility _lfingerselect "Collapsed")))
  (if (Math|Conversions|ToBoolean(Integer) _rfinger)
    (Variables|/Script/UMG.Widget|SetVisibility _rfingerselect "Visible")
    (bind _returnvalue_3 (Class|TextBox|GetFingerPosX true _rfinger))
    (bind _returnvalue_4 (Class|TextBox|GetFingerPosY true _rfinger))
    (Class|CanvasPanelSlot|SetPosition (Class|WidgetLayoutLibrary|SlotasCanvasSlot _rfingerselect) (Math|Vector2D|MakeVector2D (Math|Conversions|ToFloat(Integer) _returnvalue_3) (Math|Conversions|ToFloat(Integer) _returnvalue_4)))
    (else
      (Variables|/Script/UMG.Widget|SetVisibility _rfingerselect "Collapsed"))))

(event EventResetKeys
  (bind _wbprobottext (Variables|Default|GetWBPRobotText))
  (Default|ResetKeys _wbprobottext)
  (Variables|/Script/UMG.Widget|SetVisibility (Variables|/Game/HUD/RobotTextBox/WBP_RobotTextBox.WBP_RobotTextBox_C|GetLFingerSelect _wbprobottext) "Collapsed")
  (Variables|/Script/UMG.Widget|SetVisibility (Variables|/Game/HUD/RobotTextBox/WBP_RobotTextBox.WBP_RobotTextBox_C|GetRFingerSelect _wbprobottext) "Collapsed"))

(event EventResetInput
  (Variables|/Script/UMG.EditableText|SetText (Variables|/Game/HUD/TouchTypingTextInput/WBP_TouchTypingTextInput.WBP_TouchTypingTextInput_C|GetRawInput (stale EventBeginPlay _returnvalue)) "")
  (Variables|Default|SetInput ""))

(event EventFinishLesson
  (bind _robottext (Variables|Default|Getrobottext))
  (bind _wbprobottext (Variables|Default|GetWBPRobotText))
  (if (>= (+ (Variables|Default|Getmistakes) (Variables|Default|Getcrtmistakes)) 20)
    (|SetBy-RefVar (Utilities|Array|Get(acopy) (Variables|/Script/FoxRacing.RobotTextBox|GetScript (Utilities|ResolveSoftReference _robottext)) (Variables|/Script/FoxRacing.RobotTextBox|GetscriptIndex (Utilities|ResolveSoftReference _robottext))) "You have made too many mistakes. Press Esc and try again.")
    (Class|RobotTextBox|Print (Utilities|ResolveSoftReference _robottext))
    (Variables|/Script/UMG.Widget|SetVisibility (stale EventBeginPlay _returnvalue) "Collapsed")
    (Variables|Default|Setlfinger 0)
    (Variables|Default|Setrfinger 0)
    (else
      (Class|RobotTextBox|Print (Utilities|ResolveSoftReference _robottext))
      (Variables|/Script/UMG.Widget|SetVisibility (stale EventBeginPlay _returnvalue) "Collapsed")
      (bind _asbp_game_progress (Utilities|Casting|CastToBP_GameProgress (Game|GetGameInstance)))
      (Math|Integer|IncrementInt (Variables|/Game/Blueprints/BP_GameProgress.BP_GameProgress_C|Getlesson _asbp_game_progress)
        (:%20%20
          (Variables|Default|Setlfinger 0)
          (Variables|Default|Setrfinger 0)))))
  (Default|ResetKeys _wbprobottext)
  (Variables|/Script/UMG.Widget|SetVisibility (Variables|/Game/HUD/RobotTextBox/WBP_RobotTextBox.WBP_RobotTextBox_C|GetLFingerSelect _wbprobottext) "Collapsed")
  (Variables|/Script/UMG.Widget|SetVisibility (Variables|/Game/HUD/RobotTextBox/WBP_RobotTextBox.WBP_RobotTextBox_C|GetRFingerSelect _wbprobottext) "Collapsed"))

(fn ConstructionScript)