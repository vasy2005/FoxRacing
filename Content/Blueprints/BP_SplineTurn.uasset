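; BP_SplineTurn is a turn track segment that moves the fox along a spline at typing speed, existing only in game Mode 2.
; A Timeline sets the fox's transform along the spline, then passes movement and direction to the next BP_SplineForward.
; Each update scales play rate by BP_TextBox WPM and spline length, switching idle and gallop animations.
; BeginPlay scatters random fruit along the spline; FReverse toggles travel direction mid-run.
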(event Custom|FReverse
  (bind _fox (Variables|Default|Getfox))
  (bind _output_get (Variables|Default|Setreverse (not (Variables|Default|Getreverse))))
  (if _output_get
    (bind _returnvalue (Class|SplineTurn|GetSplineForward))
    (Variables|/Script/FoxRacing.SplineForward|Setreverse _returnvalue (not (Variables|/Script/FoxRacing.SplineForward|Getreverse _returnvalue)))
    (bind _track (Timeline|Timeline Reverse)
      (:Update
        (Transformation|SetActorTransform (Utilities|ResolveSoftReference _fox) (Math|Transform|MakeTransform (Spline|GetLocationatDistanceAlongSpline (Variables|Default|GetSpline) (Math|Float|Lerp 0.0 (Spline|GetSplineLength (Variables|Default|GetSpline)) _track) "World") (Spline|GetRotationatDistanceAlongSpline (Variables|Default|GetSpline) (Math|Float|Lerp 0.0 (Spline|GetSplineLength (Variables|Default|GetSpline)) _track) "World") "1.000000,1.000000,1.000000"))
        (if (Variables|Default|Getreverse)
          (Class|Actor|AddActorWorldRotation (Utilities|ResolveSoftReference _fox) "0.000000,180.000000,0.000000"))
        (CallFunction|Update))
      (:Finished
        (bind _returnvalue_2 (Class|SplineTurn|GetSplineForwardReverse))
        (bind _returnvalue_3 (Class|SplineTurn|GetSplineForward))
        (bind _asbp_spline_forward (Utilities|Casting|CastToBP_SplineForward _returnvalue_3))
        (Variables|/Script/FoxRacing.SplineForward|Setreverse _asbp_spline_forward _returnvalue_2)
        (Default|Move _asbp_spline_forward)))
    (else
      (Timeline|Timeline Play))))

(event Custom|Move
  (bind _fox (Variables|Default|Getfox))
  (Components|Timeline|SetPlayRate (Variables|Default|GetTimeline) 0.2)
  (if (Variables|Default|Getreverse)
    (bind _track (Timeline|Timeline ReverseFromEnd)
      (:Update
        (Transformation|SetActorTransform (Utilities|ResolveSoftReference _fox) (Math|Transform|MakeTransform (Spline|GetLocationatDistanceAlongSpline (Variables|Default|GetSpline) (Math|Float|Lerp 0.0 (Spline|GetSplineLength (Variables|Default|GetSpline)) _track) "World") (Spline|GetRotationatDistanceAlongSpline (Variables|Default|GetSpline) (Math|Float|Lerp 0.0 (Spline|GetSplineLength (Variables|Default|GetSpline)) _track) "World") "1.000000,1.000000,1.000000"))
        (if (Variables|Default|Getreverse)
          (Class|Actor|AddActorWorldRotation (Utilities|ResolveSoftReference _fox) "0.000000,180.000000,0.000000"))
        (CallFunction|Update))
      (:Finished
        (bind _returnvalue (Class|SplineTurn|GetSplineForwardReverse))
        (bind _returnvalue_2 (Class|SplineTurn|GetSplineForward))
        (bind _asbp_spline_forward (Utilities|Casting|CastToBP_SplineForward _returnvalue_2))
        (Variables|/Script/FoxRacing.SplineForward|Setreverse _asbp_spline_forward _returnvalue)
        (Default|Move _asbp_spline_forward)))
    (else
      (Timeline|Timeline PlayFromStart))))

(event Custom|Update
  (bind _returnvalue (Actor|GetActorOfClass "/Game/Blueprints/BP_TextBox.BP_TextBox_C"))
  (bind _returnvalue_2 (Class|Spline|GetSpeed (Variables|/Script/FoxRacing.TextBox|GetWPM _returnvalue)))
  (Components|Timeline|SetPlayRate (Variables|Default|GetTimeline) (/ (* (Variables|/Script/FoxRacing.TextBox|GetWPM _returnvalue) _returnvalue_2) (Spline|GetSplineLength (Variables|Default|GetSpline))))
  (if (< (Variables|/Script/FoxRacing.TextBox|GetWPM _returnvalue) 1e+01)
    (if (Variables|Default|Getanim1)
      (bind _returnvalue_3 (Actor|GetActorOfClass "/Game/Blueprints/BP_Fox.BP_Fox_C"))
      (Components|Animation|PlayAnimation (Variables|/Game/Blueprints/BP_Fox.BP_Fox_C|GetSkeletalMesh _returnvalue_3) "/Game/Meshes/Fox/Fox_Anim_AnimalArmature_Idle_AnimalArmature.Fox_Anim_AnimalArmature_Idle_AnimalArmature" true)
      (Variables|Default|Setanim1 false)
      (Variables|Default|Setanim2 true))
    (elif (Variables|Default|Getanim2)
      (bind _returnvalue_4 (Actor|GetActorOfClass "/Game/Blueprints/BP_Fox.BP_Fox_C"))
      (Components|Animation|PlayAnimation (Variables|/Game/Blueprints/BP_Fox.BP_Fox_C|GetSkeletalMesh _returnvalue_4) "/Game/Meshes/Fox/Fox_Anim_AnimalArmature_Gallop_AnimalArmature.Fox_Anim_AnimalArmature_Gallop_AnimalArmature" true)
      (Variables|Default|Setanim1 true)
      (Variables|Default|Setanim2 false))))

(event Custom|FruitSpawn
  (for _index (range 1 (Math|Random|RandomIntegerinRange 0 (Math|Float|Truncate (/ (Spline|GetSplineLength (Variables|Default|GetSpline)) 2e+03))))
    (CallFunction|MakeFruit)))

(event Custom|Make%20Fruit
  (Game|SpawnActorfromClass "/Game/Blueprints/BP_Fruit.BP_Fruit_C" (Math|Conversions|ToTransform(Vector) (Spline|GetLocationatDistanceAlongSpline (Variables|Default|GetSpline) (Math|Float|Lerp 0.0 (Spline|GetSplineLength (Variables|Default|GetSpline)) (Math|Random|RandomFloatinRange 0.0 1.0)) "World")) "Undefined" "MultiplyWithRoot" 0 (Math|Random|RandomIntegerinRange 1 6) 0))

(event Collision|EventActorBeginOverlap
  (params (OtherActor :type Actor%20Object%20Reference)))

(event EventBeginPlay
  (Variables|Default|Setspl (Variables|Default|GetSpline))
  (CallFunction|FruitSpawn)
  (Development|PrintString "SPAWNED")
  (Variables|Default|Setanim1 true)
  (Variables|Default|Setanim2 true)
  (bind _asbp_game_progress (Utilities|Casting|CastToBP_GameProgress (Game|GetGameInstance)))
  (if (not (== (Variables|/Game/Blueprints/BP_GameProgress.BP_GameProgress_C|Getmode _asbp_game_progress) 2))
    (Actor|DestroyActor)))

(fn ConstructionScript)