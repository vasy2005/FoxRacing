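; BP_Enemy is an enemy actor that exists only when the game instance's Mode is 1, and destroys itself otherwise.
; On BeginPlay in that mode it adds a WBP_ProgressBar widget to the viewport and calls SetMesh.
; SetMesh uses the Level stored in BP_GameProgress to make one of six animal components visible, from Donkey through Wolf.
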(event Custom|Set%20Mesh
  (switch int (Variables|/Game/Blueprints/BP_GameProgress.BP_GameProgress_C|Getlevel (stale EventBeginPlay _asbp_game_progress))
    (:1
      (Variables|Default|Setskeleton (Variables|Default|GetDonkey)))
    (:2
      (Variables|Default|Setskeleton (Variables|Default|GetHorse)))
    (:3
      (Variables|Default|Setskeleton (Variables|Default|GetHusky)))
    (:4
      (Variables|Default|Setskeleton (Variables|Default|GetDeer)))
    (:5
      (Variables|Default|Setskeleton (Variables|Default|GetStag)))
    (:6
      (Variables|Default|Setskeleton (Variables|Default|GetWolf))))
  (Rendering|SetVisibility (Variables|Default|Getskeleton) true false))

(event EventBeginPlay
  (bind _asbp_game_progress (Utilities|Casting|CastToBP_GameProgress (Game|GetGameInstance)))
  (if (== (Variables|/Game/Blueprints/BP_GameProgress.BP_GameProgress_C|Getmode _asbp_game_progress) 1)
    (bind _returnvalue (UserInterface|CreateWidget "/Game/HUD/Race/WBP_ProgressBar.WBP_ProgressBar_C"))
    (UserInterface|Viewport|AddtoViewport _returnvalue 0)
    (CallFunction|SetMesh)
    (Development|PrintString "Hello")
    (else
      (Actor|DestroyActor))))

(event Collision|EventActorBeginOverlap
  (params (OtherActor :type Actor%20Object%20Reference)))

(fn ConstructionScript)