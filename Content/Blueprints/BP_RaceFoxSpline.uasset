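; Spline track that drives the player's fox in a touch-typing race, kept only when game progress matches its level ID and mode.
; A Timeline moves BP_Fox along the spline for each lap, while a self-repeating Update timer sets play rate from typing WPM and switches idle/gallop animations.
; Finishing all laps advances the level, shows the win widget and calls Lose on the enemy spline; its own Lose halts the fox.
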(event Custom|Move
  (bind _newtrack_0 (Timeline|Timeline PlayFromStart)
    (:Update
      (Variables|Default|Setfoxtrack _newtrack_0)
      (Transformation|SetActorTransform (Variables|Default|GetFox) (Math|Transform|MakeTransform (Spline|GetLocationatDistanceAlongSpline (Variables|Default|GetSpline) (Math|Float|Lerp 0.0 (Spline|GetSplineLength (Variables|Default|GetSpline)) _newtrack_0) "World") (Spline|GetRotationatDistanceAlongSpline (Variables|Default|GetSpline) (Math|Float|Lerp 0.0 (Spline|GetSplineLength (Variables|Default|GetSpline)) _newtrack_0) "World") "1.000000,1.000000,1.000000")))
    (:Finished
      (bind _result (Math|Integer|IncrementInt (Variables|Default|GetloopCounter))
        (:%20%20
          (if (< _result (Variables|Default|Getlaps))
            (CallFunction|Move)
            (else
              (Math|Integer|IncrementInt (Variables|/Game/Blueprints/BP_GameProgress.BP_GameProgress_C|Getlevel (stale EventBeginPlay _asbp_game_progress))
                (:%20%20
                  (bind _foundwidgets (Widget|GetAllWidgetsOfClass "/Game/HUD/TouchTypingTextInput/WBP_TouchTypingTextInput.WBP_TouchTypingTextInput_C" true))
                  (Variables|/Script/UMG.Widget|SetVisibility (Utilities|Array|Get(acopy) _foundwidgets) "Collapsed")
                  (Class|TextBox|Reset (Utilities|ResolveSoftReference (Variables|Default|Gettext%20box)))
                  (bind _foundwidgets_2 (Widget|GetAllWidgetsOfClass "/Game/HUD/Race/WBP_Race.WBP_Race_C" true))
                  (Default|Win (Utilities|Array|Get(acopy) _foundwidgets_2))
                  (Variables|/Script/UMG.Widget|SetVisibility (Utilities|Array|Get(acopy) _foundwidgets_2) "Visible")
                  (bind _returnvalue (Actor|GetActorOfClass "/Game/Blueprints/BP_RaceEnemySpline.BP_RaceEnemySpline_C"))
                  (Default|Lose _returnvalue))))))))))

(event Custom|Update
  (bind _fox (Variables|Default|GetFox))
  (bind _text_box (Variables|Default|Gettext%20box))
  (bind _output (Utilities|ResolveSoftReference _text_box))
  (bind _wpm (Variables|/Script/FoxRacing.TextBox|GetWPM _output))
  (Development|PrintText "UPDATE")
  (if (Variables|/Script/FoxRacing.TextBox|Getstop (Utilities|ResolveSoftReference _text_box))
    _
    (else
      (bind _returnvalue (Class|RaceFoxSpline|GetSpeed _wpm))
      (Components|Timeline|SetPlayRate (Variables|Default|GetTimeline) (/ (* _wpm _returnvalue) (Spline|GetSplineLength (Variables|Default|GetSpline))))))
  (if (< _wpm 1e+01)
    (if (Variables|Default|Getanim1)
      (Components|Animation|PlayAnimation (Variables|/Game/Blueprints/BP_Fox.BP_Fox_C|GetSkeletalMesh _fox) "/Game/Meshes/Fox/Fox_Anim_AnimalArmature_Idle_AnimalArmature.Fox_Anim_AnimalArmature_Idle_AnimalArmature" true)
      (Variables|Default|Setanim1 false)
      (Variables|Default|Setanim2 true))
    (elif (Variables|Default|Getanim2)
      (Components|Animation|PlayAnimation (Variables|/Game/Blueprints/BP_Fox.BP_Fox_C|GetSkeletalMesh _fox) "/Game/Meshes/Fox/Fox_Anim_AnimalArmature_Gallop_AnimalArmature.Fox_Anim_AnimalArmature_Gallop_AnimalArmature" true)
      (Variables|Default|Setanim1 true)
      (Variables|Default|Setanim2 false)))
  (Utilities|Time|SetTimerbyFunctionName 0 "Update" 0.5))

(event Custom|Lose
  (Components|Timeline|SetPlayRate (Variables|Default|GetTimeline) 0.0)
  (Class|TextBox|Reset (Utilities|ResolveSoftReference (Variables|Default|Gettext%20box))))

(event Collision|EventActorBeginOverlap
  (params (OtherActor :type Actor%20Object%20Reference)))

(event EventBeginPlay
  (bind _asbp_game_progress (Utilities|Casting|CastToBP_GameProgress (Game|GetGameInstance)))
  (if (and (== (Variables|/Game/Blueprints/BP_GameProgress.BP_GameProgress_C|Getlevel _asbp_game_progress) (Variables|Default|GetID)) (== (Variables|/Game/Blueprints/BP_GameProgress.BP_GameProgress_C|Getmode _asbp_game_progress) 1))
    (bind _returnvalue (Actor|GetActorOfClass "/Game/Blueprints/BP_Fox.BP_Fox_C"))
    (Variables|Default|SetFox _returnvalue)
    (Components|Timeline|SetPlayRate (Variables|Default|GetTimeline) 0.0)
    (CallFunction|Move)
    (else
      (Actor|DestroyActor))))

(fn ConstructionScript)