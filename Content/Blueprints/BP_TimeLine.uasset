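; BP_TimeLine is a helper Blueprint that animates UI widget elements through timelines for a navigation arrow and a progress bar.
; Three custom events take a target widget, play rate, start and finish, then play their own timeline from the start.
; Each update lerps between the endpoints, rotating the NavSys arrow or sliding the progress bar's Fox and enemy images horizontally via their canvas slots at a fixed height.
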(event Custom|TimelineNavSys
  (params (NavSys :type WBP%20Nav%20Sys%20Object%20Reference) (Play%20Rate :type Float%20%28double-precision%29) (Start :type Float%20%28double-precision%29) (Finish :type Float%20%28double-precision%29))
  (bind _track0 (Timeline|Timeline_0 PlayFromStart)
    (:Update
      (Class|Widget|SetRenderTransformAngle (Variables|/Game/HUD/NavSys/WBP_NavSys.WBP_NavSys_C|GetArrow NavSys) (Math|Float|Lerp Start Finish _track0)))))

(event Custom|TimelineBarFox
  (params (ProgressBar :type WBP%20Progress%20Bar%20Object%20Reference) (Play%20Rate :type Float%20%28double-precision%29) (Start :type Float%20%28double-precision%29) (Finish :type Float%20%28double-precision%29))
  (bind _track0 (Timeline|Timeline1 PlayFromStart)
    (:Update
      (Class|CanvasPanelSlot|SetPosition (Class|WidgetLayoutLibrary|SlotasCanvasSlot (Variables|/Game/HUD/Race/WBP_ProgressBar.WBP_ProgressBar_C|GetFox ProgressBar)) (Math|Vector2D|MakeVector2D (Math|Float|Lerp Start Finish _track0) 52.0)))))

(event Custom|TimelineBarEnemy
  (params (ProgressBar :type WBP%20Progress%20Bar%20Object%20Reference) (Play%20Rate :type Float%20%28double-precision%29) (Start :type Float%20%28double-precision%29) (Finish :type Float%20%28double-precision%29))
  (bind _track0 (Timeline|Timeline PlayFromStart)
    (:Update
      (Class|CanvasPanelSlot|SetPosition (Class|WidgetLayoutLibrary|SlotasCanvasSlot (Variables|/Game/HUD/Race/WBP_ProgressBar.WBP_ProgressBar_C|GetenemyImg ProgressBar)) (Math|Vector2D|MakeVector2D (Math|Float|Lerp Start Finish _track0) 52.0)))))

(event EventBeginPlay)

(event Collision|EventActorBeginOverlap
  (params (OtherActor :type Actor%20Object%20Reference)))

(event EventTick
  (params (DeltaSeconds :type Float%20%28single-precision%29)))

(fn ConstructionScript)