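; BP_Fox is an actor, apparently the player's fox, that collects fruit and adds a navigation widget on BeginPlay.
; It also shows a free-roam tutorial when the game instance's mode and new flag call for it.
; Any overlap plays a sound and increments the game-instance fruit count before the fruit cast.
; Confirmed fruit is destroyed, and a name-based timer later spawns another through CrtForward or CrtTurn, chosen by Forward.
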(event Custom|NewFruit
  (if (Variables|Default|Getforward)
    (Default|MakeFruit (Variables|Default|GetCrtForward))
    (else
      (Default|MakeFruit (Variables|Default|GetCrtTurn))))
  (Development|PrintString "NEW FRUIT"))

(event Collision|EventActorBeginOverlap
  (params (OtherActor :type Actor%20Object%20Reference))
  (Audio|SpawnSound2D "/Game/Misc/short-success-sound-glockenspiel-treasure-video-game-6346.short-success-sound-glockenspiel-treasure-video-game-6346" 1.0 1.0 0.0 0)
  (bind _asbp_game_progress (Utilities|Casting|CastToBP_GameProgress (Game|GetGameInstance)))
  (bind _result (Math|Integer|IncrementInt (Variables|/Game/Blueprints/BP_GameProgress.BP_GameProgress_C|Getfruits _asbp_game_progress))
    (:%20%20
      (Development|PrintString (Utilities|String|ToString(Integer) _result))
      (bind _asbp_fruit (Utilities|Casting|CastToBP_Fruit OtherActor))
      (Actor|DestroyActor _asbp_fruit)
      (Utilities|Time|SetTimerbyFunctionName 0 "NewFruit" 1e+01))))

(event EventBeginPlay
  (bind _returnvalue (UserInterface|CreateWidget "/Game/HUD/NavSys/WBP_NavSys.WBP_NavSys_C"))
  (UserInterface|Viewport|AddtoViewport _returnvalue 0)
  (bind _asbp_game_progress (Utilities|Casting|CastToBP_GameProgress (Game|GetGameInstance)))
  (if (and (== (Variables|/Game/Blueprints/BP_GameProgress.BP_GameProgress_C|Getmode _asbp_game_progress) 2) (Variables|/Game/Blueprints/BP_GameProgress.BP_GameProgress_C|Getnew2 _asbp_game_progress))
    (bind _returnvalue_2 (UserInterface|CreateWidget "/Game/HUD/Tutorial/WBP_TutorialFreeRoam.WBP_TutorialFreeRoam_C"))
    (UserInterface|Viewport|AddtoViewport _returnvalue_2 0)))

(fn ConstructionScript)