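; BP_RobotTextBox is an actor that starts a lesson script and shows it through the WBP_RobotTextBox widget.
; On BeginPlay it derives the lesson index from BP_GameProgress, creates and focuses the widget, then calls functions for Ro and Eng scripts and applies the result.
; Lesson1 then resets the script index and calls Print.
; Enter1 and Enter0 set the Enter flag and forward the click state to the widget.
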(event Custom|Lesson1
  (Variables|Default|SetscriptIndex 0)
  (Class|RobotTextBox|Print))

(event EventBeginPlay
  (bind _asbp_game_progress (Utilities|Casting|CastToBP_GameProgress (Game|GetGameInstance)))
  (Variables|Default|SetCrtLesson (- (Variables|/Game/Blueprints/BP_GameProgress.BP_GameProgress_C|Getlesson _asbp_game_progress) 1))
  (bind _returnvalue (UserInterface|CreateWidget "/Game/HUD/RobotTextBox/WBP_RobotTextBox.WBP_RobotTextBox_C"))
  (UserInterface|Viewport|AddtoViewport _returnvalue 0)
  (Widget|SetKeyboardFocus _returnvalue)
  (Class|RobotTextBox|LessonScriptRo (Variables|Default|GetCrtLesson))
  (Class|RobotTextBox|LessonScriptEng (Variables|Default|GetCrtLesson))
  (Class|RobotTextBox|ApplyLessonScript)
  (CallFunction|Lesson1))

(event Collision|EventActorBeginOverlap
  (params (OtherActor :type Actor%20Object%20Reference)))

(event EventTick
  (params (DeltaSeconds :type Float%20%28single-precision%29)))

(event EventEnter1
  (Variables|Default|Setenter true)
  (Default|ClickEnter1 (stale EventBeginPlay _returnvalue)))

(event EventEnter0
  (Variables|Default|Setenter false)
  (Default|ClickEnter0 (stale EventBeginPlay _returnvalue)))

(fn ConstructionScript)