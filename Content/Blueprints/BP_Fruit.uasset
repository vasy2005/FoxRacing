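; BP_Fruit is an actor that displays one of six fruit meshes as a floating, spinning pickup-style object.
; On BeginPlay, ChosenFruit selects the component (watermelon slice, apple, pear, orange, green apple or grapes), which is made visible.
; A looping SinWave timeline, started at a random time offset, then drives that fruit's relative height and yaw for a bobbing, rotating motion.
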(event Custom|SinMotion
  (Components|Timeline|SetNewTime (Variables|Default|GetSinWave) (Math|Random|RandomFloatinRange 0.0 5.0))
  (bind (_direction _sinwave _rotation) (Timeline|SinWave Play)
    (:Update
      (Transformation|SetRelativeLocationAndRotation (Variables|Default|GetCrtFruit) (Math|Vector|MakeVector 0.0 0.0 (Math|Float|Lerp 5e+01 2e+02 _sinwave)) (Math|Rotator|MakeRotator 0.0 0.0 (Math|Float|Lerp 0.0 3.6e+02 _rotation)) false false))
    (:Finished
      (Components|Timeline|PlayfromStart (Variables|Default|GetSinWave)))))

(event EventBeginPlay
  (switch int (Variables|Default|GetChosenFruit)
    (:1
      (Variables|Default|SetCrtFruit (Variables|Default|GetSlice_of_Watermelon)))
    (:2
      (Variables|Default|SetCrtFruit (Variables|Default|GetApple)))
    (:3
      (Variables|Default|SetCrtFruit (Variables|Default|GetPear)))
    (:4
      (Variables|Default|SetCrtFruit (Variables|Default|GetOrange)))
    (:5
      (Variables|Default|SetCrtFruit (Variables|Default|GetApple_Green)))
    (:6
      (Variables|Default|SetCrtFruit (Variables|Default|GetGrapes))))
  (Rendering|SetVisibility (Variables|Default|GetCrtFruit) true false)
  (CallFunction|SinMotion))

(event Collision|EventActorBeginOverlap
  (params (OtherActor :type Actor%20Object%20Reference)))

(event EventTick
  (params (DeltaSeconds :type Float%20%28single-precision%29)))

(fn ConstructionScript)