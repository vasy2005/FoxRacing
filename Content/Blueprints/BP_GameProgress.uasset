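; BP_GameProgress holds the player's progress (fruits, level, lesson, best WPM, music and two "New" values) and persists it through BP_SaveGame.
; NewSave creates a save object, while SaveGame reuses the cached one; both copy the current values into it and write slot "save0".
; LoadGame reads that slot, caches the object and copies its values back, stopping if the cast fails.
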(event Custom|NewSave
  (bind _returnvalue (SaveGame|CreateSaveGameObject "/Game/Blueprints/BP_SaveGame.BP_SaveGame_C"))
  (bind _output_get (Variables|Default|SetSave _returnvalue))
  (Variables|/Game/Blueprints/BP_SaveGame.BP_SaveGame_C|Setfruits _output_get (Variables|Default|Getfruits))
  (Variables|/Game/Blueprints/BP_SaveGame.BP_SaveGame_C|Setlevel _output_get (Variables|Default|Getlevel))
  (Variables|/Game/Blueprints/BP_SaveGame.BP_SaveGame_C|Setlesson _output_get (Variables|Default|Getlesson))
  (Variables|/Game/Blueprints/BP_SaveGame.BP_SaveGame_C|Setnew _output_get (Variables|Default|Getnew))
  (Variables|/Game/Blueprints/BP_SaveGame.BP_SaveGame_C|Setnew2 _output_get (Variables|Default|Getnew2))
  (Variables|/Game/Blueprints/BP_SaveGame.BP_SaveGame_C|Setmaxwpm _output_get (Variables|Default|Getmaxwpm))
  (Variables|/Game/Blueprints/BP_SaveGame.BP_SaveGame_C|Setmusic _output_get (Variables|Default|Getmusic))
  (SaveGame|SaveGametoSlot (Variables|Default|GetSave) "save0"))

(event Custom|SaveGame
  (bind _save (Variables|Default|GetSave))
  (Variables|/Game/Blueprints/BP_SaveGame.BP_SaveGame_C|Setfruits _save (Variables|Default|Getfruits))
  (Variables|/Game/Blueprints/BP_SaveGame.BP_SaveGame_C|Setlevel _save (Variables|Default|Getlevel))
  (Variables|/Game/Blueprints/BP_SaveGame.BP_SaveGame_C|Setlesson _save (Variables|Default|Getlesson))
  (Variables|/Game/Blueprints/BP_SaveGame.BP_SaveGame_C|Setnew _save (Variables|Default|Getnew))
  (Variables|/Game/Blueprints/BP_SaveGame.BP_SaveGame_C|Setmaxwpm _save (Variables|Default|Getmaxwpm))
  (Variables|/Game/Blueprints/BP_SaveGame.BP_SaveGame_C|Setnew2 _save (Variables|Default|Getnew2))
  (Variables|/Game/Blueprints/BP_SaveGame.BP_SaveGame_C|Setmusic _save (Variables|Default|Getmusic))
  (SaveGame|SaveGametoSlot (Variables|Default|GetSave) "save0"))

(event Custom|LoadGame
  (bind _returnvalue (SaveGame|LoadGamefromSlot "save0"))
  (bind _asbp_save_game (Utilities|Casting|CastToBP_SaveGame _returnvalue))
  (bind _output_get (Variables|Default|SetSave _asbp_save_game))
  (Variables|Default|Setfruits (Variables|/Game/Blueprints/BP_SaveGame.BP_SaveGame_C|Getfruits _output_get))
  (Variables|Default|Setlevel (Variables|/Game/Blueprints/BP_SaveGame.BP_SaveGame_C|Getlevel _output_get))
  (Variables|Default|Setlesson (Variables|/Game/Blueprints/BP_SaveGame.BP_SaveGame_C|Getlesson _output_get))
  (Variables|Default|Setnew (Variables|/Game/Blueprints/BP_SaveGame.BP_SaveGame_C|Getnew _output_get))
  (Variables|Default|Setmaxwpm (Variables|/Game/Blueprints/BP_SaveGame.BP_SaveGame_C|Getmaxwpm _output_get))
  (Variables|Default|Setnew2 (Variables|/Game/Blueprints/BP_SaveGame.BP_SaveGame_C|Getnew2 _output_get))
  (Variables|Default|Setmusic (Variables|/Game/Blueprints/BP_SaveGame.BP_SaveGame_C|Getmusic _output_get)))